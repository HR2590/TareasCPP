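; BP_ActorExample is an example actor that exercises the float attribute API of its AttributeExample member.
; On BeginPlay it checks whether an attribute exists, creates it with an initial value, then checks again and reads it back.
; It then sets and reads values under a second name, which is never created here, and under the original name, printing each check and read result.
; The construction script is empty.
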(event EventBeginPlay
  (bind _returnvalue (Class|AttributeComponent|HasAttributeFloat (Variables|Default|GetAttributeExample) (Variables|Default|GetIn%20Name)))
  (Development|PrintString (Utilities|String|ToString(Boolean) _returnvalue))
  (Class|AttributeComponent|CreateAttributeFloat (Variables|Default|GetAttributeExample) (Variables|Default|GetIn%20Name) (Variables|Default|GetIn%20Initial%20Value))
  (bind _returnvalue_2 (Class|AttributeComponent|HasAttributeFloat (Variables|Default|GetAttributeExample) (Variables|Default|GetIn%20Name)))
  (Development|PrintString (Utilities|String|ToString(Boolean) _returnvalue_2))
  (bind _returnvalue_3 (Class|AttributeComponent|GetAttributeValueFloat (Variables|Default|GetAttributeExample) (Variables|Default|GetIn%20Name)))
  (Development|PrintString (Utilities|String|ToString(Float) _returnvalue_3))
  (Class|AttributeComponent|SetAttributeValueFloat (Variables|Default|GetAttributeExample) (Variables|Default|GetIn%20Name_0) (Variables|Default|GetIn%20Value))
  (bind _returnvalue_4 (Class|AttributeComponent|GetAttributeValueFloat (Variables|Default|GetAttributeExample) (Variables|Default|GetIn%20Name_0)))
  (Development|PrintString (Utilities|String|ToString(Float) _returnvalue_4))
  (Class|AttributeComponent|SetAttributeValueFloat (Variables|Default|GetAttributeExample) (Variables|Default|GetIn%20Name) (Variables|Default|GetIn%20Value_0))
  (bind _returnvalue_5 (Class|AttributeComponent|GetAttributeValueFloat (Variables|Default|GetAttributeExample) (Variables|Default|GetIn%20Name)))
  (Development|PrintString (Utilities|String|ToString(Float) _returnvalue_5)))

(event Collision|EventActorBeginOverlap
  (params (OtherActor :type Actor%20Object%20Reference)))

(event EventTick
  (params (DeltaSeconds :type Float%20%28single-precision%29)))

(fn ConstructionScript)